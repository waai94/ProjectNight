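; Rifle fire component that spawns a projectile when firing starts on its owning gun.
; OnStartFireBP casts the owner to GunBase and spawns one scaled-down BP_BulletBase slightly ahead of the gun mesh's origin, facing along the mesh's rotation.
; The spawn ignores collisions, and the component itself has no repeat-fire or Tick logic.
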(event EventBeginPlay)

(event EventTick
  (params (DeltaSeconds :type Float%20%28single-precision%29)))

(event EventOnStartFireBP
  (bind _asgun_base (Utilities|Casting|CastToGunBase (Components|GetOwner)))
  (Game|SpawnActorfromClass "/Game/Blueprints/Bullets/BP_BulletBase.BP_BulletBase_C" (Math|Transform|MakeTransform (+ (Transformation|GetWorldLocation (Variables|/Script/CplusFastest.GunBase|GetGunMesh _asgun_base)) (* (Math|Vector|GetForwardVector (Transformation|GetWorldRotation (Variables|/Script/CplusFastest.GunBase|GetGunMesh _asgun_base))) 5e+01)) (Transformation|GetWorldRotation (Variables|/Script/CplusFastest.GunBase|GetGunMesh _asgun_base)) "0.100000,0.100000,0.100000") "AlwaysSpawn" "MultiplyWithRoot" 0 0))